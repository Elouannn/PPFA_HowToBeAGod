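; BP_PlayerPawn is a player pawn that pans along the world X and Y axes and zooms its camera, with a visible mouse cursor.
; BeginPlay adds the MC_Player Enhanced Input mapping context and enables mouse-over events.
; Directional inputs set a fixed step vector that Move adds to the actor location, without sweep or delta-time scaling.
; Zoom inputs feed MoveCam, which shifts the camera's relative height within clamped limits.
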(event `self.ReceiveBeginPlay`
  (bind _returnvalue (`GameplayStatics.GetPlayerController` 0))
  (bind _returnvalue_2 (pcsubsystem `EnhancedInputLocalPlayerSubsystem` _returnvalue))
  (`/Engine/EditorBlueprintResources/StandardMacros.IsValid` _returnvalue_2
    (:`Is Valid`
      (`EnhancedInputSubsystemInterface.AddMappingContext` _returnvalue_2 "/Game/MesDossiers/Player/Input/MC_Player.MC_Player" 0 (struct))
      (set `PlayerController.bShowMouseCursor` true _returnvalue)
      (set `PlayerController.bEnableMouseOverEvents` true _returnvalue))))

(event `EnhancedInput|/Game/MesDossiers/Player/Input/Input_Forward`
  (params (ActionValue :type Boolean) (ElapsedSeconds :type "Float (double-precision)") (TriggeredSeconds :type "Float (double-precision)") (InputAction :type "InputAction Object Reference" :default "/Game/MesDossiers/Player/Input/Input_Forward.Input_Forward"))
  (:`Triggered`
    (set `self.MoveVector` (5.0 0.0 0.0))
    (`self.Move` (`self.MoveVector`) :!label _label)))

(event `EnhancedInput|/Game/MesDossiers/Player/Input/Input_Back`
  (params (ActionValue :type Boolean) (ElapsedSeconds :type "Float (double-precision)") (TriggeredSeconds :type "Float (double-precision)") (InputAction :type "InputAction Object Reference" :default "/Game/MesDossiers/Player/Input/Input_Back.Input_Back"))
  (:`Triggered`
    (set `self.MoveVector` (-5.0 0.0 0.0))
    (goto _label)))

(event `Move`
  (params (NewParam :type "Vector Structure"))
  (`self.K2_SetActorLocation` (+ NewParam (`self.K2_GetActorLocation`))))

(event `EnhancedInput|/Game/MesDossiers/Player/Input/Input_Left`
  (params (ActionValue :type Boolean) (ElapsedSeconds :type "Float (double-precision)") (TriggeredSeconds :type "Float (double-precision)") (InputAction :type "InputAction Object Reference" :default "/Game/MesDossiers/Player/Input/Input_Left.Input_Left"))
  (:`Triggered`
    (set `self.MoveVector` (0.0 -5.0 0.0))
    (goto _label)))

(event `EnhancedInput|/Game/MesDossiers/Player/Input/Input_Right`
  (params (ActionValue :type Boolean) (ElapsedSeconds :type "Float (double-precision)") (TriggeredSeconds :type "Float (double-precision)") (InputAction :type "InputAction Object Reference" :default "/Game/MesDossiers/Player/Input/Input_Right.Input_Right"))
  (:`Triggered`
    (set `self.MoveVector` (0.0 5.0 0.0))
    (goto _label)))

(event `EnhancedInput|/Game/MesDossiers/Player/Input/Input_ZoomIn`
  (params (ActionValue :type Boolean) (ElapsedSeconds :type "Float (double-precision)") (TriggeredSeconds :type "Float (double-precision)") (InputAction :type "InputAction Object Reference" :default "/Game/MesDossiers/Player/Input/Input_ZoomIn.Input_ZoomIn"))
  (:`Triggered`
    (set `self.CamHeightModif` -20.0)
    (`self.MoveCam` (`self.CamHeightModif`) :!label _label_2)))

(event `MoveCam`
  (params (NewParam :type "Float (double-precision)"))
  (bind _camera (`self.Camera`))
  (bind (_relativelocation_x _relativelocation_y _relativelocation_z) (`KismetMathLibrary.BreakVector` (`SceneComponent.RelativeLocation` _camera)))
  (`SceneComponent.K2_SetRelativeLocation` _camera (`KismetMathLibrary.MakeVector` _relativelocation_x _relativelocation_y (`KismetMathLibrary.FClamp` (+ NewParam _relativelocation_z) 200.0 800.0)) false false))

(event `EnhancedInput|/Game/MesDossiers/Player/Input/Input_ZoomOut`
  (params (ActionValue :type Boolean) (ElapsedSeconds :type "Float (double-precision)") (TriggeredSeconds :type "Float (double-precision)") (InputAction :type "InputAction Object Reference" :default "/Game/MesDossiers/Player/Input/Input_ZoomOut.Input_ZoomOut"))
  (:`Triggered`
    (set `self.CamHeightModif` 20.0)
    (goto _label_2)))

(fn `UserConstructionScript`)