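; Village AI manager that spawns villagers at the town hall, tracks shared food and wood, and assigns villager tasks.
; FindATask writes a blackboard Task target, prioritizing low food, then low wood, then affordable construction, with missing-resource gathering and TownHall as fallbacks.
; Gather lookups reserve the first free spot with a navigable path and prune invalid ones.
; It registers itself on BP_Player and updates the village stats widget.
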(event `SpawnPnj`
  (params (PnjCount :type Integer))
  (`self.SpawnPnjMacro` PnjCount))

(event `self.ReceiveBeginPlay`
  (bind _asbp_player (cast `/Game/MyAssets/MainBP/BP_Player` (`GameplayStatics.GetPlayerPawn` 0)))
  (set `/Game/MyAssets/MainBP/BP_Player.AI_Manager` self _asbp_player)
  (bind _returnvalue (`|CreateWidget` "/Game/MyAssets/PNJ/AITask/WB_VillageStats.WB_VillageStats_C"))
  (bind _output_get (set `self.WB_VillageStats` _returnvalue))
  (`UserWidget.AddToViewport` _output_get 0)
  (`self.SetRessources` _output_get)
  (`self.SpawnPnjMacro` (`self.BeginPnjNumber`)))

(event `PnjDeath`
  (params (AIToKill :type "/Game/MyAssets/PNJ/BP_VillagerParent Object Reference"))
  (`self.PnjDeathUI`)
  (`self.K2_DestroyActor` AIToKill))

(fn `AddRessource`
  (params (Ressource :type "/Game/MyAssets/MainBP/Data/Enum_RessourceEnd Enum" :default "NewEnumerator0") (Number :type Integer))
  (switch `/Game/MyAssets/MainBP/Data/Enum_RessourceEnd` Ressource
    (:`NewEnumerator0`
      (set `self.Food` (+ Number (`self.Food`))))
    (:`NewEnumerator1`
      (set `self.Wood` (+ Number (`self.Wood`)))))
  (`self.SetRessources` (`self.WB_VillageStats`))
  (return))

(fn `BuildTask`)

(fn `FindATask`
  (params (Villager :type "/Game/MyAssets/PNJ/BP_VillagerParent Object Reference"))
  (locals (NewLocalVar :type "/Game/MyAssets/MainBP/Enviro/BP_RessourceParent Object Reference"))
  (`self.CheckStats`
    (:`LowFood`
      (bind _ressource (`self.GetFoodTask`)
        (:`RessourceAvailable`
          (set `local.NewLocalVar` _ressource))
        (:`RessourceNotavailable`
          (bind _ressource_2 (`self.GetWoodTask` :!label _label)
            (:`RessourceAvailable`
              (set `local.NewLocalVar` _ressource_2))
            (:`RessourceNotavailable`
              (bind (_battobuild _missingfood _missingwood) (`self.ConstructionOrder` :!label _label_2)
                (:`Output`
                  (set `local.NewLocalVar` _battobuild))
                (:`NoBuildPossible`
                  (if _missingfood
                    (bind _ressource_3 (`self.GetFoodTask`)
                      (:`RessourceAvailable`
                        (set `local.NewLocalVar` _ressource_3))
                      (:`RessourceNotavailable`
                        (if _missingwood :!label _label_3
                          (bind _ressource_4 (`self.GetWoodTask`)
                            (:`RessourceAvailable`
                              (set `local.NewLocalVar` _ressource_4))
                            (:`RessourceNotavailable`
                              (set `local.NewLocalVar` (`self.TownHall`) :!label _label_4)))
                          (else
                            (goto _label_4)))))
                    (else
                      (goto _label_3))))))))))
    (:`LowWood`
      (goto _label))
    (:`BothGood`
      (goto _label_2)))
  (`BlackboardComponent.SetValueAsObject` (`/Game/MyAssets/PNJ/BP_VillagerParent.Blackboard` Villager) "Task" (`local.NewLocalVar`))
  (return))

(fn `LookAtStats`)

(fn `NewPnjUI`
  (`/Game/MyAssets/PNJ/AITask/WB_VillageStats.ChangePop` (`self.WB_VillageStats`) true)
  (return))

(fn `PnjDeathUI`
  (`/Game/MyAssets/PNJ/AITask/WB_VillageStats.ChangePop` (`self.WB_VillageStats`) false)
  (return))

(fn `SetRessources`
  (params (self3 :type "/Game/MyAssets/PNJ/AITask/WB_VillageStats Object Reference"))
  (`/Game/MyAssets/PNJ/AITask/WB_VillageStats.SetFood` self3 (`self.Food`))
  (`/Game/MyAssets/PNJ/AITask/WB_VillageStats.SetWood` self3 (`self.Wood`))
  (return))

(fn `UserConstructionScript`)

(fn `WarTask`)

(fn `WoodTask`)