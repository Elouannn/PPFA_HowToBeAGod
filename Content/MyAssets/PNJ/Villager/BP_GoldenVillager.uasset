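; BP_GoldenVillager is a villager NPC Blueprint that starts its AI behavior tree when play begins.
; BeginPlay calls the parent logic, then Change BT, which casts the controller to PNJ_Controller, runs the tree and returns the result.
; Change BT ignores its NewBT input and always runs the BehaviourTree variable.
; The construction script only calls its parent.
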(event `self.ReceiveBeginPlay`
  (`parent.ReceiveBeginPlay`)
  (`self.Change BT` (`self.BehaviourTree`)))

(fn `Change BT`
  (params (NewBT :type "BehaviorTree Object Reference"))
  (returns (Success :type Boolean))
  (bind _aspnj_controller (cast `/Game/MyAssets/PNJ/PNJ_Controller` (`self.GetController`)))
  (bind _returnvalue (`AIController.RunBehaviorTree` _aspnj_controller (`self.BehaviourTree`)))
  (return _returnvalue))

(fn `UserConstructionScript`
  (`parent.UserConstructionScript`))