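; Base villager NPC for a village-management game that gathers resources and constructs buildings.
; A blackboard Task object drives the work and is shown on a text render, while start and stop calls toggle the AnimBP's Working flag.
; Resources accumulate until the stack limit, then the villager targets the TownHall to deposit them through AIManager and get a new task.
; Buildings are paid from AIManager's Food and Wood before being built.
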(event `self.ReceiveBeginPlay`
  (set `self.Blackboard` (`AIBlueprintHelperLibrary.GetBlackboard` (`self.GetController`)))
  (bind _asabp_villager (cast `/Game/MyAssets/PNJ/Villager/ABP_Villager` (`SkeletalMeshComponent.GetAnimInstance` (`self.Mesh`))))
  (set `self.As ABP Villager` _asabp_villager))

(event `self.ReceiveTick`
  (params (DeltaSeconds :type "Float (single-precision)"))
  (`TextRenderComponent.K2_SetText` (`self.TextRender`) (`KismetTextLibrary.Conv_ObjectToText` (`BlackboardComponent.GetValueAsObject` (`self.Blackboard`) "Task"))))

(event `StartRessourceTask`
  (set `/Game/MyAssets/PNJ/Villager/ABP_Villager.Working` true (`self.As ABP Villager`))
  (bind _asbp_batiment (cast `/Game/MyAssets/MainBP/Enviro/BP_Batiment` (`BlackboardComponent.GetValueAsObject` (`self.Blackboard`) "Task")))
  (if (not (`/Game/MyAssets/MainBP/Enviro/BP_Batiment.Payed` _asbp_batiment))
    (`self.PayThePrice` _asbp_batiment
      (:`PricePayed`
        (set `/Game/MyAssets/MainBP/Enviro/BP_Batiment.Payed` true _asbp_batiment)))))

(fn `StopRessourceTask`
  (bind _blackboard (`self.Blackboard`))
  (bind _ai_manager (`self.AI_Manager`))
  (bind _returnvalue (`BlackboardComponent.GetValueAsObject` _blackboard "Task"))
  (set `/Game/MyAssets/PNJ/Villager/ABP_Villager.Working` false (`self.As ABP Villager`))
  (bind _asbp_ressource_parent (cast `/Game/MyAssets/MainBP/Enviro/BP_RessourceParent` (`BlackboardComponent.GetValueAsObject` (`self.Blackboard`) "Task")))
  (bind _asbp_batiment (cast `/Game/MyAssets/MainBP/Enviro/BP_Batiment` _asbp_ressource_parent)
    (:`then`
      (if (`/Game/MyAssets/MainBP/Enviro/BP_Batiment.Payed` _asbp_batiment)
        (`/Game/MyAssets/MainBP/Enviro/BP_Batiment.BuildBat1` _asbp_batiment)
        (if (`/Game/MyAssets/MainBP/Enviro/BP_Batiment.Finished` _asbp_batiment)
          (`BlackboardComponent.SetValueAsObject` (`self.Blackboard`) "Task" null :!label _label))
        (else
          (goto _label)))
      (return))
    (:`CastFailed`
      (set `/Game/MyAssets/MainBP/Enviro/BP_RessourceParent.Occuped` false _asbp_ressource_parent)
      (bind (_collected _finished _townhall) (`/Game/MyAssets/MainBP/Enviro/BP_RessourceParent.Collect` _asbp_ressource_parent))
      (if _townhall
        (`/Game/MyAssets/PNJ/AITask/BP_AIManager.AddRessource` (`self.AI_Manager`) (`self.Final RessourceSaved`) (`self.RessourcesInHand`))
        (set `self.RessourcesInHand` 0)
        (`/Game/MyAssets/PNJ/AITask/BP_AIManager.FindATask` _ai_manager self)
        (if _finished :!label _label_2
          (`self.K2_DestroyActor` _asbp_ressource_parent)
          (`BlackboardComponent.SetValueAsObject` (`self.Blackboard`) "Task" (`/Game/MyAssets/PNJ/AITask/BP_AIManager.TownHall` (`self.AI_Manager`)))
          (return))
        (else
          (bind _output_get (set `self.RessourcesInHand` (+ _collected (`self.RessourcesInHand`))))
          (if (>= _output_get (`/Game/MyAssets/MainBP/Enviro/BP_RessourceParent.MaxStackOnVillager` _asbp_ressource_parent))
            (bind _asbp_ressource_parent_2 (cast `/Game/MyAssets/MainBP/Enviro/BP_RessourceParent` _returnvalue)
              (:`then`
                (set `self.Final RessourceSaved` (`/Game/MyAssets/MainBP/Enviro/BP_RessourceParent.FinalRessource` _asbp_ressource_parent_2))
                (set `self.SavedTask` _returnvalue)
                (`BlackboardComponent.SetValueAsObject` _blackboard "Task" (`/Game/MyAssets/PNJ/AITask/BP_AIManager.TownHall` _ai_manager))
                (goto _label_2))
              (:`CastFailed`
                (`KismetSystemLibrary.PrintString` "Warning Bug BP_VillagerParent")
                (return)))
            (else
              (goto _label_2))))))))

(fn `UserConstructionScript`)