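; BP_CollectOutpost is a collection outpost actor that wraps a BP_Maison as a child actor and registers itself with a manager.
; On BeginPlay it casts the child actor to BP_Maison, turns off that actor's collision, then adds itself to the Manager's PostDeCollect list.
; Registration happens only if the cast succeeds, and the parent BeginPlay is left unwired, so it never runs.
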(event `self.ReceiveBeginPlay`
  (bind _asbp_maison (cast `/Game/MyAssets/MainBP/Village/BP_Maison` (`ChildActorComponent.ChildActor` (`self.ChildActor`))))
  (`self.SetActorEnableCollision` _asbp_maison false)
  (`KismetArrayLibrary.Array_Add` (`/Game/MyAssets/PNJ/AITask/BP_AIManager.PostDeCollect` (`self.Manager`)) self))

(fn `UserConstructionScript`
  (`parent.UserConstructionScript`))