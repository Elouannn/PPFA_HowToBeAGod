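; Base Blueprint for harvestable resources, which villagers collect from.
; On BeginPlay it fills its name, image, total, per-tick yield and villager stack limit from a data table row keyed by its resource enum.
; Collect deducts a clamped per-tick amount and reports depletion, except on Town Hall instances, which it only flags.
; Helper functions set or clear green and red translucent overlay materials on the mesh.
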(event `self.ReceiveBeginPlay`
  (bind _returnvalue (`|GetDataTableRow` (`self.DataTableRessource`) (`KismetStringLibrary.Conv_StringToName` (`|GetEnumeratorNameAsString` (`self.Ressource`))))
    (:`then`
      (bind (_ressourcename _finalressource _image _totalressource _collectpertick _maxstackonvillager) (break `/Game/MyAssets/MainBP/Data/Struct_RessourceTask` _returnvalue))
      (set `self.RessourceName` _ressourcename)
      (set `self.FinalRessource` _finalressource)
      (set `self.Image` _image)
      (set `self.TotalRessource` _totalressource)
      (set `self.CollectPerTick` _collectpertick)
      (set `self.MaxStackOnVillager` _maxstackonvillager))))

(fn `Collect`
  (returns (Collected :type Integer) (Finished :type Boolean) (TownHall :type Boolean))
  (locals (NewLocalVar :type Boolean) (NewLocalVar_0 :type Boolean))
  (bind _totalressource (`self.TotalRessource`))
  (bind _collectpertick (`self.CollectPerTick`))
  (set `local.NewLocalVar_0` false)
  (set `local.NewLocalVar` false)
  (cast `/Game/MyAssets/MainBP/Enviro/BP_TownHall` self
    (:`then`
      (set `local.NewLocalVar_0` true))
    (:`CastFailed`
      (if (< _totalressource _collectpertick)
        (set `self.CollectPerTick` _totalressource))
      (set `self.TotalRessource` (- _totalressource _collectpertick))
      (set `local.NewLocalVar` (<= (`self.TotalRessource`) 0))))
  (return (`self.CollectPerTick`) (`local.NewLocalVar`) (`local.NewLocalVar_0`)))

(fn `ColorGreen`
  (`MeshComponent.SetOverlayMaterial` (`self.Mesh`) "/Game/MyAssets/MainBP/Materials/MI_Translucent_Green.MI_Translucent_Green")
  (return))

(fn `ColorRed`
  (`MeshComponent.SetOverlayMaterial` (`self.Mesh`) "/Game/MyAssets/MainBP/Materials/MI_Translucent_Red.MI_Translucent_Red")
  (return))

(fn `NoColor`
  (`MeshComponent.SetOverlayMaterial` (`self.Mesh`) null)
  (return))

(fn `UserConstructionScript`)