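; BP_Batiment is a constructible building whose Walls mesh reflects its state: unpaid, paid or finished.
; Each BuildBat1 call adds HP and refreshes the mesh, then marks it Finished at HPMax and runs FinishBuild to reveal the walls and enable collision once.
; MajLooking runs before the Finished check, so that call still shows the previous shape.
; ClearSite spawns and activates a BP_Pouvoir1 at the mesh transform, only once.
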(event `self.ReceiveBeginPlay`
  (`parent.ReceiveBeginPlay`)
  (`self.MajLooking`))

(event `FinishBuild`
  (bind _walls (`self.Walls`))
  (`/Engine/EditorBlueprintResources/StandardMacros.DoOnce` false
    (:`Completed`
      (`PrimitiveComponent.SetCollisionEnabled` _walls "QueryAndPhysics")
      (`SceneComponent.SetHiddenInGame` _walls false false))))

(event `MajLooking`
  (bind _walls (`self.Walls`))
  (bind _shapes (`self.Shapes`))
  (if (`self.Finished`)
    (`StaticMeshComponent.SetStaticMesh` _walls (`|GetArrayItem` _shapes 2))
    (elif (`self.Payed`)
      (`StaticMeshComponent.SetStaticMesh` _walls (`|GetArrayItem` _shapes 1))
      (else
        (`StaticMeshComponent.SetStaticMesh` _walls (`|GetArrayItem` _shapes))))))

(event `ClearSite`
  (`/Engine/EditorBlueprintResources/StandardMacros.DoOnce` false
    (:`Completed`
      (bind _returnvalue (`|SpawnActorFromClass` "/Game/MyAssets/MainBP/Pouvoirs/BP_Pouvoir1.BP_Pouvoir1_C" (`SceneComponent.K2_GetComponentToWorld` (`self.Mesh`)) "Undefined" "MultiplyWithRoot" null null))
      (`/Game/MyAssets/MainBP/Pouvoirs/BP_PouvoirParent.Activate` _returnvalue))))

(fn `BuildBat1`
  (bind _output_get (set `self.HP` (+ (`self.HP`) 10)))
  (`self.MajLooking`)
  (if (>= _output_get (`self.HPMax`))
    (set `self.Finished` true)
    (`self.FinishBuild`))
  (return))

(fn `UserConstructionScript`
  (`parent.UserConstructionScript`))