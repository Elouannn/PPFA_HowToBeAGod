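; BP_SpawnerAnimals is a placed spawner that creates animals when activated.
; Activate fires once through a DoOnce, spawning a BP_PouvoirSpawnANimaux at the spawner's location and calling ForceSpawn with its Animal and Number values.
; If Condition is true, it also plays a dialogue line on the player's HUD widget, then destroys itself.
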(event `Activate`
  (`/Engine/EditorBlueprintResources/StandardMacros.DoOnce` false
    (:`Completed`
      (bind _returnvalue (`|SpawnActorFromClass` "/Game/MyAssets/MainBP/Pouvoirs/BP_PouvoirSpawnANimaux.BP_PouvoirSpawnANimaux_C" (`KismetMathLibrary.MakeTransform` (`self.K2_GetActorLocation`)) "Undefined" "MultiplyWithRoot" null null))
      (`/Game/MyAssets/MainBP/Pouvoirs/BP_PouvoirSpawnANimaux.ForceSpawn` _returnvalue (`self.Animal`) (`self.Number`))
      (if (`self.Condition`)
        (bind _asbp_player (cast `/Game/MyAssets/MainBP/BP_Player` (`GameplayStatics.GetPlayerPawn` 0)))
        (`/Game/MyAssets/MainBP/Widget/WB_HUD.PlayDialogue` (`/Game/MyAssets/MainBP/BP_Player.WidgetHUD` _asbp_player) 8)
        (`self.K2_DestroyActor`)))))

(fn `UserConstructionScript`)