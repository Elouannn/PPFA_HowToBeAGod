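; Parent Blueprint for animals that react to villagers, flee or fight, and can burn to death.
; BeginPlay loads stats from DT_Animaux by animal type, and sphere overlap interrupts villagers and sets walk speed.
; StartFight drives Blackboard keys: zero-damage animals flee temporarily, others target the attacker.
; A looping burn timer, stopped by water, feeds TakeDamage and the HP widget; burn death spawns food registered with the AI manager.
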(event `self.ReceiveBeginPlay`
  ;[1 1 1] Begin Play
  (bind _asbp_player (cast `/Game/MyAssets/MainBP/BP_Player` (`GameplayStatics.GetPlayerPawn` 0)))
  (set `self.As BP Player` _asbp_player)
  (bind _aswb_hpanimaux (cast `/Game/MyAssets/MainBP/Widget/WB_HPAnimaux` (`WidgetComponent.GetWidget` (`self.Widget`))))
  (set `self.As WB HPAnimaux` _aswb_hpanimaux)
  (bind _returnvalue (`|GetDataTableRow` "/Game/MyAssets/MainBP/Data/DT_Animaux.DT_Animaux" (`KismetStringLibrary.Conv_StringToName` (`|GetEnumeratorNameAsString` (`self.AnimalType`))))
    (:`then`
      (bind (_type _maxhp _damage _foodtodrop _corpsmort) (break `/Game/MyAssets/MainBP/Data/Struct_Animaux` _returnvalue))
      (bind _output_get (set `self.HPMax` _maxhp))
      (set `self.HP` _output_get)
      (set `self.Damage` _damage)
      (set `self.Food to Drop` _foodtodrop)
      (set `self.Corps Mort` _corpsmort)
      (`SphereComponent.SetSphereRadius` (`self.Sphere`) 200.0 true))))

(event `self.Sphere.OnComponentBeginOverlap`
  (params (OverlappedComponent :type "PrimitiveComponent Object Reference") (OtherActor :type "Actor Object Reference") (OtherComp :type "PrimitiveComponent Object Reference") (OtherBodyIndex :type Integer) (bFromSweep :type Boolean) (SweepResult :type "HitResult Structure (by ref)"))
  ;[1 1 1] Begin Overlap large
  (bind _asbp_villager_parent (cast `/Game/MyAssets/PNJ/BP_VillagerParent` OtherActor))
  (`/Game/MyAssets/PNJ/BP_VillagerParent.GetInterupted` _asbp_villager_parent "NewEnumerator6" self null)
  (set `CharacterMovementComponent.MaxWalkSpeed` 350.0 (`self.CharacterMovement`)))

(event `AfficherUI`
  (bind _widget (`self.Widget`))
  ;[0.4034 0.7537 1] Afficher UI
  (`SceneComponent.SetHiddenInGame` _widget false false)
  (`KismetSystemLibrary.RetriggerableDelay` 3.0)
  (`/Engine/EditorBlueprintResources/StandardMacros.IsValid` _widget
    (:`Is Valid`
      (`SceneComponent.SetHiddenInGame` _widget false false))))

(event `/Game/MyAssets/MainBP/Enviro/BPI_Bruler.Bruler`
  (params (Feu :type "/Game/MyAssets/MainBP/Enviro/BP_Feu Object Reference") (Water :type Boolean))
  (bind _feuchild (`self.FeuChild`))
  (bind _burntimer (`self.BurnTimer`))
  ;[1 0.7606 0.2396] Bruler
  (if Water
    (if (`KismetSystemLibrary.K2_IsValidTimerHandle` _burntimer)
      (`KismetSystemLibrary.K2_ClearAndInvalidateTimerHandle` _burntimer)
      (`ChildActorComponent.SetChildActorClass` _feuchild null))
    (elif (== (`ChildActorComponent.ChildActor` _feuchild) null)
      (`ChildActorComponent.SetChildActorClass` _feuchild "/Game/MyAssets/MainBP/Enviro/BP_Feu.BP_Feu_C")
      (bind _returnvalue (`KismetSystemLibrary.K2_SetTimerDelegate` (delegate `Burn`) 1.0 true))
      (set `self.BurnTimer` _returnvalue))))

(event `Burn`
  ;[1 0.7606 0.2396] Bruler
  (if (== (`ChildActorComponent.ChildActorClass` (`self.FeuChild`)) "/Game/MyAssets/MainBP/Enviro/BP_Feu.BP_Feu_C")
    (bind _deadornot (`self.TakeDamage` 2))
    (if _deadornot
      (set `self.Dead` true)
      (set `self.Combat` false)
      (`KismetSystemLibrary.Delay` 1.0)
      (bind _returnvalue (`|SpawnActorFromClass` "/Game/MyAssets/MainBP/Enviro/BP_FoodParent.BP_FoodParent_C" (`KismetMathLibrary.MakeTransform` (`self.K2_GetActorLocation`)) "AlwaysSpawn" "MultiplyWithRoot" null "NewEnumerator4" "NewEnumerator0" null))
      (`KismetArrayLibrary.Array_Add` (`/Game/MyAssets/PNJ/AITask/BP_AIManager.FoodSpots` (`/Game/MyAssets/MainBP/BP_Player.AI_Manager` (`self.As BP Player`))) _returnvalue)
      (`StaticMeshComponent.SetStaticMesh` (`self.StaticMesh`) (`self.Corps Mort`))
      (`self.K2_DestroyActor`))
    (else
      (`KismetSystemLibrary.K2_ClearAndInvalidateTimerHandle` (`self.BurnTimer`)))))

(event `StartFight`
  (params (PnjTarget :type "/Game/MyAssets/PNJ/BP_VillagerParent Object Reference"))
  (bind _returnvalue (`AIBlueprintHelperLibrary.GetBlackboard` (`self.GetController`)))
  ;[0.6198 0.1001 0.1001] Start Fight
  (set `self.PNJToAvoid` null)
  (if (== (`self.Damage`) 0)
    ;;[1 1 1] Fuir
    (set `self.PNJToAvoid` PnjTarget)
    (`BlackboardComponent.SetValueAsBool` _returnvalue "Fuir" true)
    (`KismetSystemLibrary.Delay` 8.0)
    (if (`BlackboardComponent.GetValueAsBool` _returnvalue "Fuir")
      (`BlackboardComponent.SetValueAsBool` _returnvalue "Fuir" false))
    (else
      ;;[1 1 1] Se Battre
      (`/Engine/EditorBlueprintResources/StandardMacros.IsValid` (`self.Pnj Target`)
        (:`Is Not Valid`
          (bind _output_get (set `self.Pnj Target` PnjTarget))
          (`BlackboardComponent.SetValueAsObject` _returnvalue "FightTarget" _output_get))))))

(fn `DealDamage`)

(fn `TakeDamage`
  (params (Damage :type Integer))
  (returns (DeadOrNot :type Boolean))
  (bind _output_get (set `self.HP` (- (`self.HP`) Damage)))
  (`ProgressBar.SetPercent` (`/Game/MyAssets/MainBP/Widget/WB_HPAnimaux.ProgressBar_0` (`self.As WB HPAnimaux`)) (/ (`self.HP`) (`self.HPMax`)))
  (`|ExecutionSequence`
    (:`then_0`
      (`self.AfficherUI`))
    (:`then_1`
      (return (<= _output_get 0)))))

(fn `UserConstructionScript`)