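; Economy component that manages the money spent on divine power spells held by the player.
; BuySpell refunds any held power, looks up the requested one in DT_PouvoirDivins and, if affordable, spawns it under the cursor as PowerInHand and deducts its price.
; CancelActualSpell refunds the held power's price and destroys it.
; The player pawn is cached on BeginPlay.
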(event `self.ReceiveBeginPlay`
  (bind _asbp_player (cast `/Game/MyAssets/MainBP/BP_Player` (`GameplayStatics.GetPlayerPawn` 0)))
  (set `self.Player` _asbp_player))

(fn `BuySpell`
  (params (ObjectToBuy :type Integer))
  (returns (Bought :type Boolean))
  (locals (TempBool :type Boolean))
  (`/Engine/EditorBlueprintResources/StandardMacros.IsValid` (`/Game/MyAssets/MainBP/BP_Player.PowerInHand` (`self.Player`))
    (:`Is Valid`
      (`self.CancelActualSpell`))
    (:`Is Not Valid`
      _))
  (bind _returnvalue (`|GetDataTableRow` "/Game/MyAssets/MainBP/Data/DT_PouvoirDivins.DT_PouvoirDivins" (`KismetStringLibrary.Conv_StringToName` (`KismetStringLibrary.Conv_IntToString` ObjectToBuy)))
    (:`then`
      (bind (_name _price _mesh _self) (break `/Game/MyAssets/MainBP/Data/DataStruct_PouvoirDivins` _returnvalue))
      (bind _output_get (set `self.PriceToPay` _price))
      (if (>= (`self.Money`) _output_get)
        (bind _output_get_2 (set `local.TempBool` true))
        (`KismetSystemLibrary.PrintString` (`KismetStringLibrary.Conv_BoolToString` _output_get_2))
        (bind _returnvalue_2 (`|SpawnActorFromClass` _self (`KismetMathLibrary.MakeTransform` (`.Location` (`GameplayStatics.BreakHitResult` (`PlayerController.GetHitResultUnderCursorByChannel` (`/Game/MyAssets/MainBP/BP_Player.PC_Player` (`self.Player`)) "TraceTypeQuery1" true)))) "Undefined" "MultiplyWithRoot" null null))
        (set `/Game/MyAssets/MainBP/BP_Player.PowerInHand` _returnvalue_2 (`self.Player`))
        (set `self.Money` (- (`self.Money`) (`self.PriceToPay`)))
        (else
          (bind _output_get_3 (set `local.TempBool` false))
          (`KismetSystemLibrary.PrintString` (`KismetStringLibrary.Conv_BoolToString` _output_get_3))))
      (return (`local.TempBool`)))))

(fn `CancelActualSpell`
  (bind _powerinhand (`/Game/MyAssets/MainBP/BP_Player.PowerInHand` (`self.Player`)))
  (`/Engine/EditorBlueprintResources/StandardMacros.IsValid` _powerinhand
    (:`Is Valid`
      (set `self.Money` (+ (`self.Money`) (`.Price_7_C8115398410D9F2218B6BA9B0282D75E` (break `/Game/MyAssets/MainBP/Data/DataStruct_PouvoirDivins` (`/Game/MyAssets/MainBP/Pouvoirs/BP_PouvoirParent.DataRow` _powerinhand)))))
      (`Actor.K2_DestroyActor` _powerinhand)
      (set `/Game/MyAssets/MainBP/BP_Player.PowerInHand` null (`self.Player`)))
    (:`Is Not Valid`
      _))
  (return))