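; BP_NavMeshBlocker is an actor in the FogOfWar folder that places its Cube, presumably a navmesh blocker, on the ground.
; On BeginPlay it multi-line traces straight down from the Cube on the Visibility channel and looks for a hit actor with the display name "LeSol".
; It moves the Cube to the first such hit, or destroys itself when none is found.
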(event `self.ReceiveBeginPlay`
  (bind _returnvalue (`SceneComponent.K2_GetComponentLocation` (`self.Cube`)))
  (bind _outhits (`KismetSystemLibrary.LineTraceMulti` _returnvalue (`KismetMathLibrary.MakeVector` (.x _returnvalue) (.y _returnvalue) (- (.z _returnvalue) 10000.0)) "TraceTypeQuery1"))
  (for _array_element _outhits
    (bind (_bblockinghit _binitialoverlap _time _distance _location _impactpoint _normal _impactnormal _physmat _hitactor) (`GameplayStatics.BreakHitResult` _array_element))
    (if (`KismetStringLibrary.EqualEqual_StrStr` "LeSol" (`KismetSystemLibrary.GetDisplayName` _hitactor))
      (`SceneComponent.K2_SetWorldLocation` (`self.Cube`) _location false false)
      (set `self.Once` true)
      (break)))
  (if (not (`self.Once`))
    (`self.K2_DestroyActor`)))

(fn `UserConstructionScript`)