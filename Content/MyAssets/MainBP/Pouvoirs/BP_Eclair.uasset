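; BP_Eclair is a lightning power actor that strikes everything around its spawn point once, on BeginPlay.
; A 100-unit multi-sphere trace on the Visibility channel finds the hits, with persistent debug drawing left on.
; Each villager, animal or resource hit gets a BP_Feu fire spawned at its location.
; Villagers and animals then take heavy damage, while resources run their own lightning reaction through PrendreLaFoudre.
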(event `self.ReceiveBeginPlay`
  (bind _returnvalue (`self.K2_GetActorLocation`))
  (bind _outhits (`KismetSystemLibrary.SphereTraceMulti` :`Start` _returnvalue :`End` _returnvalue :`Radius` 100.0 :`TraceChannel` "TraceTypeQuery1" :`DrawDebugType` "Persistent"))
  (for _array_element _outhits
    (bind (_bblockinghit _binitialoverlap _time _distance _location _impactpoint _normal _impactnormal _physmat _hitactor) (`GameplayStatics.BreakHitResult` _array_element))
    (bind _asbp_villager (cast `/Game/MyAssets/PNJ/Villager/BP_Villager` _hitactor)
      (:`then`
        (`|SpawnActorFromClass` "/Game/MyAssets/MainBP/Enviro/BP_Feu.BP_Feu_C" (`KismetMathLibrary.MakeTransform` (`self.K2_GetActorLocation` _asbp_villager)) "Undefined" "MultiplyWithRoot" null null)
        (`/Game/MyAssets/PNJ/BP_VillagerParent.LoseHP` _asbp_villager 500 null))
      (:`CastFailed`
        (bind _asbp_animaux_parent (cast `/Game/MyAssets/MainBP/Animaux/BP_AnimauxParent` _hitactor)
          (:`then`
            (`|SpawnActorFromClass` "/Game/MyAssets/MainBP/Enviro/BP_Feu.BP_Feu_C" (`KismetMathLibrary.MakeTransform` (`self.K2_GetActorLocation` _asbp_animaux_parent)) "Undefined" "MultiplyWithRoot" null null)
            (`/Game/MyAssets/MainBP/Animaux/BP_AnimauxParent.TakeDamage` _asbp_animaux_parent 500))
          (:`CastFailed`
            (bind _asbp_ressource_parent (cast `/Game/MyAssets/MainBP/Enviro/BP_RessourceParent` _hitactor))
            (`|SpawnActorFromClass` "/Game/MyAssets/MainBP/Enviro/BP_Feu.BP_Feu_C" (`KismetMathLibrary.MakeTransform` (`self.K2_GetActorLocation` _asbp_ressource_parent)) "Undefined" "MultiplyWithRoot" null null)
            (`/Game/MyAssets/MainBP/Enviro/BP_RessourceParent.PrendreLaFoudre` _asbp_ressource_parent)))))))

(fn `UserConstructionScript`)