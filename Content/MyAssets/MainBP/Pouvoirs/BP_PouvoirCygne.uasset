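; BP_PouvoirCygne is a swan power actor that interrupts nearby villagers when activated.
; Activate runs a debug-drawn sphere trace around itself and looks for a finished BP_Batiment that stores Faveur, defaulting the Activateur to itself.
; It calls GetInterupted on each villager hit, passing the Activateur and an interruption type chosen by whether that is a building.
; It then hides its static mesh.
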(event `self.Activate`
  (bind _returnvalue (`self.K2_GetActorLocation`))
  (bind _activateur (`self.Activateur`))
  (set `self.Activateur` self)
  (bind _outhits (`KismetSystemLibrary.SphereTraceMulti` :`Start` _returnvalue :`End` _returnvalue :`Radius` 800.0 :`TraceChannel` "TraceTypeQuery1" :`DrawDebugType` "ForDuration" :`DrawTime` 1.0))
  (for _array_element _outhits
    (bind _asbp_batiment (cast `/Game/MyAssets/MainBP/Enviro/BP_Batiment` (`.HitActor` (`GameplayStatics.BreakHitResult` _array_element))))
    (switch `/Game/MyAssets/MainBP/Data/Enum_RessourceEnd` (`/Game/MyAssets/MainBP/Enviro/BP_Batiment.Ressource AStocker` _asbp_batiment)
      (:`NewEnumerator5`
        (if (`/Game/MyAssets/MainBP/Enviro/BP_Batiment.Finished` _asbp_batiment)
          (set `self.Activateur` _asbp_batiment)
          (break)))))
  (for _array_element_2 _outhits
    (bind _asbp_villager_parent (cast `/Game/MyAssets/PNJ/BP_VillagerParent` (`.HitActor` (`GameplayStatics.BreakHitResult` _array_element_2))))
    (if (== _activateur "/Game/MyAssets/MainBP/Enviro/BP_Batiment.BP_Batiment")
      (`/Game/MyAssets/PNJ/BP_VillagerParent.GetInterupted` _asbp_villager_parent "NewEnumerator9" _activateur null)
      (else
        (`/Game/MyAssets/PNJ/BP_VillagerParent.GetInterupted` _asbp_villager_parent "NewEnumerator10" _activateur null))))
  (`SceneComponent.SetHiddenInGame` (`self.StaticMesh`) true false))

(fn `UserConstructionScript`
  (`parent.UserConstructionScript`))