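; BP_PouvoirFoudre is a lightning power actor that, on Activate, calls down a short burst of BP_Eclair lightning actors around itself.
; It hides its mesh and, after a brief delay, spawns the first bolt at its own location.
; The SpawnEclair macro is then chained four times, each waiting a random delay before spawning another bolt at a random navigable point within a fixed radius.
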(event `self.Activate`
  (`SceneComponent.SetVisibility` (`self.StaticMesh`) false false)
  (`KismetSystemLibrary.Delay` 0.2)
  (`|SpawnActorFromClass` "/Game/MyAssets/MainBP/Pouvoirs/BP_Eclair.BP_Eclair_C" (`KismetMathLibrary.MakeTransform` (`self.K2_GetActorLocation`)) "Undefined" "MultiplyWithRoot" null null)
  (`self.SpawnEclair`
    (:`NewParam2`
      (`self.SpawnEclair`
        (:`NewParam2`
          (`self.SpawnEclair`
            (:`NewParam2`
              (`self.SpawnEclair`))))))))

(fn `UserConstructionScript`
  (`parent.UserConstructionScript`))