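; BP_PouvoirPluie is a rain power actor.
; Its Activate event spawns a BP_Pluie at the actor's own location, then destroys the power actor.
; A disconnected sphere trace around the mesh that would destroy BP_Feu fire actors is left in the graph and never runs.
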(event `self.Activate`
  (`|SpawnActorFromClass` "/Game/MyAssets/MainBP/Pouvoirs/BP_Pluie.BP_Pluie_C" (`KismetMathLibrary.MakeTransform` (`self.K2_GetActorLocation`)) "Undefined" "MultiplyWithRoot" null null)
  (`self.K2_DestroyActor`))

(event `self.ReceiveTick`
  (params (DeltaSeconds :type "Float (single-precision)"))
  (`parent.ReceiveTick` DeltaSeconds))

(fn `UserConstructionScript`
  (`parent.UserConstructionScript`))