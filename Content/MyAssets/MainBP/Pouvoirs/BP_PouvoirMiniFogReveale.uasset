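; Mini fog-reveal power actor that unlocks the buildings, resources and spawners in a small area.
; Its mesh overlaps preview the area by tinting unstarted resources green.
; Activate hides the mesh and sphere-traces around the actor, registering construction sites and new food or wood spots with the player's AIManager, destroying nav mesh blockers and triggering animal spawners.
; It then plays a brief Niagara effect and destroys itself.
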(event `self.ReceiveBeginPlay`
  (`parent.ReceiveBeginPlay`))

(event `self.Activate`
  (bind _ns_pouvoir1_0 (`self.NS_Pouvoir1_0`))
  (bind _returnvalue (`SceneComponent.K2_GetComponentLocation` (`self.DefaultSceneRoot`)))
  (`SceneComponent.SetHiddenInGame` (`self.StaticMesh`) true false)
  (bind _outhits (`KismetSystemLibrary.SphereTraceMulti` _returnvalue _returnvalue 500.0 "TraceTypeQuery1"))
  (for _array_element _outhits
    (bind (_bblockinghit _binitialoverlap _time _distance _location _impactpoint _normal _impactnormal _physmat _hitactor) (`GameplayStatics.BreakHitResult` _array_element))
    (bind _asbp_ressource_parent (cast `/Game/MyAssets/MainBP/Enviro/BP_RessourceParent` _hitactor)
      (:`then`
        (bind _asbp_batiment (cast `/Game/MyAssets/MainBP/Enviro/BP_Batiment` _hitactor)
          (:`then`
            (bind _asbp_player (cast `/Game/MyAssets/MainBP/BP_Player` (`GameplayStatics.GetPlayerPawn` 0)))
            (`KismetArrayLibrary.Array_Add` (`/Game/MyAssets/PNJ/AITask/BP_AIManager.ConstructionSites` (`/Game/MyAssets/MainBP/BP_Player.AI_Manager` _asbp_player)) _asbp_batiment)
            (`/Game/MyAssets/MainBP/Enviro/BP_Batiment.MajLooking` _asbp_batiment)
            (`SceneComponent.SetHiddenInGame` (`/Game/MyAssets/MainBP/Enviro/BP_Batiment.ChildActor` _asbp_batiment) false false)
            (`SceneComponent.SetHiddenInGame` (`/Game/MyAssets/MainBP/Enviro/BP_Batiment.BuildSpot` _asbp_batiment) true false)
            (`/Game/MyAssets/MainBP/Enviro/BP_Batiment.ClearSite` _asbp_batiment))
          (:`CastFailed`
            (`/Game/MyAssets/MainBP/Enviro/BP_RessourceParent.NoColor` _asbp_ressource_parent)
            (if (not (`/Game/MyAssets/MainBP/Enviro/BP_RessourceParent.Started` _asbp_ressource_parent))
              (set `/Game/MyAssets/MainBP/Enviro/BP_RessourceParent.Started` true _asbp_ressource_parent)
              (bind _asbp_player_2 (cast `/Game/MyAssets/MainBP/BP_Player` (`GameplayStatics.GetPlayerPawn` 0)))
              (switch `/Game/MyAssets/MainBP/Data/Enum_RessourceEnd` (`/Game/MyAssets/MainBP/Enviro/BP_RessourceParent.FinalRessource` _asbp_ressource_parent)
                (:`NewEnumerator0`
                  (bind _asbp_food_parent (cast `/Game/MyAssets/MainBP/Enviro/BP_FoodParent` _asbp_ressource_parent))
                  (bind _ai_manager (`/Game/MyAssets/MainBP/BP_Player.AI_Manager` _asbp_player_2))
                  (`KismetArrayLibrary.Array_Add` (`/Game/MyAssets/PNJ/AITask/BP_AIManager.FoodSpots` _ai_manager) _asbp_food_parent))
                (:`NewEnumerator1`
                  (bind _asbp_wood_parent (cast `/Game/MyAssets/MainBP/Enviro/BP_WoodParent` _asbp_ressource_parent))
                  (`KismetArrayLibrary.Array_Add` (`/Game/MyAssets/PNJ/AITask/BP_AIManager.WoodSpots` _ai_manager) _asbp_wood_parent)))))))
      (:`CastFailed`
        (bind _asbp_nav_mesh_blocker (cast `/Game/MyAssets/MainBP/FogOfWar/BP_NavMeshBlocker` _hitactor)
          (:`then`
            (`self.K2_DestroyActor` _asbp_nav_mesh_blocker))
          (:`CastFailed`
            (bind _asbp_spawner_animals (cast `/Game/MyAssets/MainBP/Animaux/BP_SpawnerAnimals` _hitactor))
            (`/Game/MyAssets/MainBP/Animaux/BP_SpawnerAnimals.Activate` _asbp_spawner_animals))))))
  (`ActorComponent.Activate` _ns_pouvoir1_0 false)
  (`KismetSystemLibrary.Delay` 1.0)
  (`ActorComponent.Deactivate` _ns_pouvoir1_0)
  (`self.K2_DestroyActor`))

(event `self.StaticMesh.OnComponentBeginOverlap`
  (params (OverlappedComponent :type "PrimitiveComponent Object Reference") (OtherActor :type "Actor Object Reference") (OtherComp :type "PrimitiveComponent Object Reference") (OtherBodyIndex :type Integer) (bFromSweep :type Boolean) (SweepResult :type "HitResult Structure (by ref)"))
  (bind _asbp_ressource_parent (cast `/Game/MyAssets/MainBP/Enviro/BP_RessourceParent` OtherActor))
  (if (not (`/Game/MyAssets/MainBP/Enviro/BP_RessourceParent.Started` _asbp_ressource_parent))
    (`/Game/MyAssets/MainBP/Enviro/BP_RessourceParent.ColorGreen` _asbp_ressource_parent)))

(event `self.StaticMesh.OnComponentEndOverlap`
  (params (OverlappedComponent :type "PrimitiveComponent Object Reference") (OtherActor :type "Actor Object Reference") (OtherComp :type "PrimitiveComponent Object Reference") (OtherBodyIndex :type Integer))
  (bind _asbp_ressource_parent (cast `/Game/MyAssets/MainBP/Enviro/BP_RessourceParent` OtherActor))
  (`/Game/MyAssets/MainBP/Enviro/BP_RessourceParent.NoColor` _asbp_ressource_parent))

(fn `UserConstructionScript`
  (`parent.UserConstructionScript`))