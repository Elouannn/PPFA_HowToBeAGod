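; A placeable power actor that pairs two nearby villagers to make a baby.
; While its mesh overlaps villagers, those with a low enough interruption level get a green overlay, cleared when the overlap ends.
; On Activate, a sphere trace gathers eligible villagers and interrupts the first two, each naming the other as activator.
; With fewer than two it prints a warning; either way the actor then destroys itself.
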(event `self.Activate`
  (bind _as_bp_villager_parent (`self.As BP Villager Parent`))
  (bind _returnvalue (`SceneComponent.K2_GetComponentLocation` (`self.StaticMesh`)))
  (bind _output (`|GetArrayItem` _as_bp_villager_parent))
  (bind _output_2 (`|GetArrayItem` _as_bp_villager_parent 1))
  (`KismetArrayLibrary.Array_Clear` (`self.As BP Villager Parent`))
  (bind _outhits (`KismetSystemLibrary.SphereTraceMulti` _returnvalue _returnvalue 400.0 "TraceTypeQuery1"))
  (for _array_element _outhits
    (bind _asbp_villager_parent (cast `/Game/MyAssets/PNJ/BP_VillagerParent` (`.HitActor` (`GameplayStatics.BreakHitResult` _array_element))))
    (if (< (`/Game/MyAssets/PNJ/BP_VillagerParent.InteruptionLevel` _asbp_villager_parent) 2)
      (`KismetArrayLibrary.Array_Add` (`self.As BP Villager Parent`) _asbp_villager_parent)))
  (if (>= (`KismetArrayLibrary.Array_Length` _as_bp_villager_parent) 2)
    (`/Game/MyAssets/PNJ/BP_VillagerParent.GetInterupted` _output "NewEnumerator4" _output_2 null)
    (`/Game/MyAssets/PNJ/BP_VillagerParent.GetInterupted` _output_2 "NewEnumerator4" _output null)
    (else
      (`KismetSystemLibrary.PrintString` "Need 2 peoples to make baby")))
  (`self.K2_DestroyActor`))

(event `self.StaticMesh.OnComponentBeginOverlap`
  (params (OverlappedComponent :type "PrimitiveComponent Object Reference") (OtherActor :type "Actor Object Reference") (OtherComp :type "PrimitiveComponent Object Reference") (OtherBodyIndex :type Integer) (bFromSweep :type Boolean) (SweepResult :type "HitResult Structure (by ref)"))
  (bind _asbp_villager_parent (cast `/Game/MyAssets/PNJ/BP_VillagerParent` OtherActor))
  (if (< (`/Game/MyAssets/PNJ/BP_VillagerParent.InteruptionLevel` _asbp_villager_parent) 2)
    (`MeshComponent.SetOverlayMaterial` (`Character.Mesh` _asbp_villager_parent) "/Game/MyAssets/MainBP/Materials/MI_Translucent_Green.MI_Translucent_Green")))

(event `self.StaticMesh.OnComponentEndOverlap`
  (params (OverlappedComponent :type "PrimitiveComponent Object Reference") (OtherActor :type "Actor Object Reference") (OtherComp :type "PrimitiveComponent Object Reference") (OtherBodyIndex :type Integer))
  (bind _asbp_villager_parent (cast `/Game/MyAssets/PNJ/BP_VillagerParent` OtherActor))
  (`MeshComponent.SetOverlayMaterial` (`Character.Mesh` _asbp_villager_parent) null))

(fn `UserConstructionScript`
  (`parent.UserConstructionScript`))