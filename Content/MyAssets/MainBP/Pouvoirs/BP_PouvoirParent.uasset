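; BP_PouvoirParent is the base actor for divine powers, providing a mesh and cursor-following placement.
; On BeginPlay it caches the PC_Player controller and sets its static mesh from the DT_PouvoirDivins row named by RowName.
; While Condition is true, Tick moves the actor to the Visibility trace hit under the cursor.
; The Activate event is empty here, apparently a hook for child powers.
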(event `self.ReceiveBeginPlay`
  (bind _aspc_player (cast `/Game/MyAssets/MainBP/PC_Player` (`GameplayStatics.GetPlayerController` 0)))
  (set `self.PC` _aspc_player)
  (bind _returnvalue (`|GetDataTableRow` "/Game/MyAssets/MainBP/Data/DT_PouvoirDivins.DT_PouvoirDivins" (`self.Row Name`))
    (:`then`
      (bind _output_get (set `self.DataRow` _returnvalue))
      (`StaticMeshComponent.SetStaticMesh` (`self.StaticMesh`) (`.Mesh_8_B962DF3F4676683D90924489D21AB0F4` (break `/Game/MyAssets/MainBP/Data/DataStruct_PouvoirDivins` _output_get))))))

(event `self.ReceiveTick`
  (params (DeltaSeconds :type "Float (single-precision)"))
  (if (`self.Condition`)
    (`self.K2_SetActorLocation` (`.Location` (`GameplayStatics.BreakHitResult` (`PlayerController.GetHitResultUnderCursorByChannel` (`self.PC`) "TraceTypeQuery1" true))))))

(event `Activate`)

(fn `UserConstructionScript`)