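; BP_PouvoirWar is a war power actor that sends the player's living NPCs to fight animals in a targeted area.
; While its mesh overlaps animals, it tints them with a translucent green overlay material.
; On Activate, a stationary multi-sphere trace gathers nearby animals into an enemy list.
; It then interrupts every living NPC from the player's AIManager with a random fight target from that list, and destroys itself.
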(event `self.Activate`
  (bind _ennemilist (`self.EnnemiList`))
  (bind _returnvalue (`SceneComponent.K2_GetComponentLocation` (`self.StaticMesh`)))
  (`KismetArrayLibrary.Array_Clear` (`self.EnnemiList`))
  (bind _outhits (`KismetSystemLibrary.SphereTraceMulti` _returnvalue _returnvalue 400.0 "TraceTypeQuery1"))
  (for _array_element _outhits
    (bind _asbp_animaux_parent (cast `/Game/MyAssets/MainBP/Animaux/BP_AnimauxParent` (`.HitActor` (`GameplayStatics.BreakHitResult` _array_element))))
    (`KismetArrayLibrary.Array_Add` _ennemilist _asbp_animaux_parent))
  (bind _asbp_player (cast `/Game/MyAssets/MainBP/BP_Player` (`GameplayStatics.GetPlayerPawn` 0)))
  (for _array_element_2 (`/Game/MyAssets/PNJ/AITask/BP_AIManager.LivingPnjListe` (`/Game/MyAssets/MainBP/BP_Player.AI_Manager` _asbp_player))
    (`/Game/MyAssets/PNJ/BP_VillagerParent.GetInterupted` _array_element_2 "NewEnumerator14" null (`KismetArrayLibrary.Array_Random` _ennemilist)))
  (`self.K2_DestroyActor`))

(event `self.StaticMesh.OnComponentBeginOverlap`
  (params (OverlappedComponent :type "PrimitiveComponent Object Reference") (OtherActor :type "Actor Object Reference") (OtherComp :type "PrimitiveComponent Object Reference") (OtherBodyIndex :type Integer) (bFromSweep :type Boolean) (SweepResult :type "HitResult Structure (by ref)"))
  (bind _asbp_animaux_parent (cast `/Game/MyAssets/MainBP/Animaux/BP_AnimauxParent` OtherActor))
  (`MeshComponent.SetOverlayMaterial` (`Character.Mesh` _asbp_animaux_parent) "/Game/MyAssets/MainBP/Materials/MI_Translucent_Green.MI_Translucent_Green"))

(event `self.StaticMesh.OnComponentEndOverlap`
  (params (OverlappedComponent :type "PrimitiveComponent Object Reference") (OtherActor :type "Actor Object Reference") (OtherComp :type "PrimitiveComponent Object Reference") (OtherBodyIndex :type Integer))
  (bind _asbp_animaux_parent (cast `/Game/MyAssets/MainBP/Animaux/BP_AnimauxParent` OtherActor))
  (`MeshComponent.SetOverlayMaterial` (`Character.Mesh` _asbp_animaux_parent) null))

(fn `UserConstructionScript`
  (`parent.UserConstructionScript`))