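; Power actor that spawns a group of animals around itself on reachable navigation points, then destroys itself.
; Activate maps the player's AnimalSpawnLevel to cumulative tier odds, rolls a tier and picks a random animal from its array, with rarer tiers generally spawning fewer.
; ForceSpawn skips the roll, taking a given animal and count.
; When QuickVariable is valid, each spawned animal is passed to its QuickEvent.
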(event `ForceSpawn`
  (params (Animal :type "/Game/MyAssets/MainBP/Animaux/BP_AnimauxParent Class Reference") (Number :type Integer) (QuickVariable :type "/Game/MyAssets/MainBP/Pouvoirs/BP_PouvoirCygne Object Reference"))
  (bind _returnvalue_location (`KismetMathLibrary.BreakTransform` (`self.GetTransform`)))
  (set `self.AnimalToSpawn` Animal)
  (set `self.AnimalNumber` Number)
  (for _ (range (`self.AnimalNumber`)) :!label _label
    (bind _returnvalue (`|SpawnActorFromClass` (`self.AnimalToSpawn`) (`KismetMathLibrary.MakeTransform` (`NavigationSystemV1.K2_GetRandomReachablePointInRadius` _returnvalue_location 150.0 null null)) "AdjustIfPossibleButAlwaysSpawn" "MultiplyWithRoot" null null))
    (`/Engine/EditorBlueprintResources/StandardMacros.IsValid` QuickVariable
      (:`Is Valid`
        (bind _asbp_animaux_parent (cast `/Game/MyAssets/MainBP/Animaux/BP_AnimauxParent` _returnvalue))
        (`/Game/MyAssets/MainBP/Pouvoirs/BP_PouvoirCygne.QuickEvent` QuickVariable _asbp_animaux_parent))))
  (`self.K2_DestroyActor`))

(event `self.Activate`
  (bind _spawnlevel (`self.SpawnLevel`))
  (bind _asbp_player (cast `/Game/MyAssets/MainBP/BP_Player` (`GameplayStatics.GetPlayerPawn` 0)))
  (switch `int` (`/Game/MyAssets/MainBP/BP_Player.AnimalSpawnLevel` _asbp_player)
    (:`0`
      (set `self.Level0Chance` 1.0)
      (set `self.Level1Chance` 0.0)
      (set `self.Level2Chance` 0.0)
      (set `self.Level3Chance` 0.0))
    (:`1`
      (set `self.Level0Chance` 0.4)
      (set `self.Level1Chance` 0.8)
      (set `self.Level2Chance` 1.0)
      (set `self.Level3Chance` 0.0))
    (:`2`
      (set `self.Level0Chance` 0.0)
      (set `self.Level1Chance` 0.4)
      (set `self.Level2Chance` 0.8)
      (set `self.Level3Chance` 1.0))
    (:`3`
      (set `self.Level0Chance` 0.0)
      (set `self.Level1Chance` 0.1)
      (set `self.Level2Chance` 0.5)
      (set `self.Level3Chance` 1.0)))
  (set `self.SpawnLevel` (`KismetMathLibrary.RandomFloatInRange` 0.0 1.0))
  (if (<= _spawnlevel (`self.Level0Chance`))
    (set `self.AnimalToSpawn` (`self.GetRandomAnimal` (`self.Animallvl0`)))
    (set `self.AnimalNumber` 3)
    (goto _label)
    (elif (<= _spawnlevel (`self.Level1Chance`))
      (set `self.AnimalToSpawn` (`self.GetRandomAnimal` (`self.Animallvl1`)))
      (set `self.AnimalNumber` 2)
      (goto _label)
      (elif (<= _spawnlevel (`self.Level2Chance`))
        (set `self.AnimalToSpawn` (`self.GetRandomAnimal` (`self.Animallvl2`)))
        (set `self.AnimalNumber` 2)
        (goto _label)
        (elif (<= _spawnlevel (`self.Level3Chance`))
          (set `self.AnimalToSpawn` (`self.GetRandomAnimal` (`self.Animallvl3`)))
          (set `self.AnimalNumber` 1)
          (goto _label))))))

(fn `GetRandomAnimal`
  (params (NewParam :type "Array of /Game/MyAssets/MainBP/Animaux/BP_AnimauxParent Class Reference"))
  (returns (NewParam1 :type "/Game/MyAssets/MainBP/Animaux/BP_AnimauxParent Class Reference"))
  (return (`|GetArrayItem` NewParam (`KismetMathLibrary.RandomIntegerInRange` 0 (- (`KismetArrayLibrary.Array_Length` NewParam) 1)))))

(fn `UserConstructionScript`
  (`parent.UserConstructionScript`))