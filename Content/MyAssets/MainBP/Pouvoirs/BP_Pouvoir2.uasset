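; BP_Pouvoir2 is a power actor that interrupts villagers within an area, then destroys itself.
; While it exists, villagers overlapping its static mesh get a translucent green overlay, cleared when the overlap ends.
; Activate runs a multi sphere trace at the mesh location and calls GetInterupted on each villager hit with a fixed enum value.
; The trace leaves persistent debug drawing, and its radius is independent of the mesh's overlap area.
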(event `self.Activate`
  (bind _returnvalue (`SceneComponent.K2_GetComponentLocation` (`self.StaticMesh`)))
  (bind _outhits (`KismetSystemLibrary.SphereTraceMulti` :`Start` _returnvalue :`End` _returnvalue :`Radius` 200.0 :`TraceChannel` "TraceTypeQuery1" :`DrawDebugType` "Persistent"))
  (for _array_element _outhits
    (bind _asbp_villager_parent (cast `/Game/MyAssets/PNJ/BP_VillagerParent` (`.HitActor` (`GameplayStatics.BreakHitResult` _array_element))))
    (`/Game/MyAssets/PNJ/BP_VillagerParent.GetInterupted` _asbp_villager_parent "NewEnumerator11"))
  (`self.K2_DestroyActor`))

(event `self.StaticMesh.OnComponentBeginOverlap`
  (params (OverlappedComponent :type "PrimitiveComponent Object Reference") (OtherActor :type "Actor Object Reference") (OtherComp :type "PrimitiveComponent Object Reference") (OtherBodyIndex :type Integer) (bFromSweep :type Boolean) (SweepResult :type "HitResult Structure (by ref)"))
  (bind _asbp_villager_parent (cast `/Game/MyAssets/PNJ/BP_VillagerParent` OtherActor))
  (`MeshComponent.SetOverlayMaterial` (`Character.Mesh` _asbp_villager_parent) "/Game/MyAssets/MainBP/Materials/MI_Translucent_Green.MI_Translucent_Green"))

(event `self.StaticMesh.OnComponentEndOverlap`
  (params (OverlappedComponent :type "PrimitiveComponent Object Reference") (OtherActor :type "Actor Object Reference") (OtherComp :type "PrimitiveComponent Object Reference") (OtherBodyIndex :type Integer))
  (bind _asbp_villager_parent (cast `/Game/MyAssets/PNJ/BP_VillagerParent` OtherActor))
  (`MeshComponent.SetOverlayMaterial` (`Character.Mesh` _asbp_villager_parent) null))

(fn `UserConstructionScript`
  (`parent.UserConstructionScript`))