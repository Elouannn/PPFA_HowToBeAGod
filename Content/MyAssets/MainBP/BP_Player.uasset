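; Player pawn for a mouse-driven game with a free-moving camera, which sets up its input mapping, cursor and HUD on BeginPlay.
; Input actions pan the pawn in fixed world-axis steps, and the mouse wheel zooms via clamped spring arm length.
; Left click activates the held power and right click cancels it through the economy component, both clearing the hand.
; A helper traces under the cursor, and a debug key sets money.
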(event Input|EnhancedActionEvents|EnhancedInputActionInputAction_MoveForward
  (params (ActionValue :type Boolean) (ElapsedSeconds :type Float%20%28double-precision%29) (TriggeredSeconds :type Float%20%28double-precision%29) (InputAction :type Input%20Action%20Object%20Reference :default "/Game/MyAssets/MainBP/Input/InputAction_MoveForward.InputAction_MoveForward"))
  (bind _returnvalue (Transformation|GetActorLocation))
  ;[1 1 1] Camera
  (Transformation|SetActorLocation (Math|Vector|MakeVector (+ (.x _returnvalue) 15.0) (.y _returnvalue) (.z _returnvalue)) false false))

(event Input|EnhancedActionEvents|EnhancedInputActionInputAction_MoveBack
  (params (ActionValue :type Boolean) (ElapsedSeconds :type Float%20%28double-precision%29) (TriggeredSeconds :type Float%20%28double-precision%29) (InputAction :type Input%20Action%20Object%20Reference :default "/Game/MyAssets/MainBP/Input/InputAction_MoveBack.InputAction_MoveBack"))
  (bind _returnvalue (Transformation|GetActorLocation))
  ;[1 1 1] Camera
  (Transformation|SetActorLocation (Math|Vector|MakeVector (- (.x _returnvalue) 15.0) (.y _returnvalue) (.z _returnvalue)) false false))

(event Input|EnhancedActionEvents|EnhancedInputActionInputAction_MoveRight
  (params (ActionValue :type Boolean) (ElapsedSeconds :type Float%20%28double-precision%29) (TriggeredSeconds :type Float%20%28double-precision%29) (InputAction :type Input%20Action%20Object%20Reference :default "/Game/MyAssets/MainBP/Input/InputAction_MoveRight.InputAction_MoveRight"))
  (bind _returnvalue (Transformation|GetActorLocation))
  ;[1 1 1] Camera
  (Transformation|SetActorLocation (Math|Vector|MakeVector (.x _returnvalue) (+ (.y _returnvalue) 15.0) (.z _returnvalue)) false false))

(event Input|EnhancedActionEvents|EnhancedInputActionInputAction_MoveLeft
  (params (ActionValue :type Boolean) (ElapsedSeconds :type Float%20%28double-precision%29) (TriggeredSeconds :type Float%20%28double-precision%29) (InputAction :type Input%20Action%20Object%20Reference :default "/Game/MyAssets/MainBP/Input/InputAction_MoveLeft.InputAction_MoveLeft"))
  (bind _returnvalue (Transformation|GetActorLocation))
  ;[1 1 1] Camera
  (Transformation|SetActorLocation (Math|Vector|MakeVector (.x _returnvalue) (- (.y _returnvalue) 15.0) (.z _returnvalue)) false false))

(event Input|EnhancedActionEvents|EnhancedInputActionInputAction_LeftClick
  (params (ActionValue :type Boolean) (ElapsedSeconds :type Float%20%28double-precision%29) (TriggeredSeconds :type Float%20%28double-precision%29) (InputAction :type Input%20Action%20Object%20Reference :default "/Game/MyAssets/MainBP/Input/InputAction_LeftClick.InputAction_LeftClick"))
  ;[1 1 1] Left click
  (if (CallFunction|ActorinHand)
    (Variables|/Game/MyAssets/MainBP/Pouvoirs/BP_PouvoirParent.BP_PouvoirParent_C|SetCondition (Variables|Default|GetPowerInHand) false)
    (Default|Activate (Variables|Default|GetPowerInHand))
    (Variables|Default|SetPowerInHand 0)))

(event Input|EnhancedActionEvents|EnhancedInputActionInputAction_RightClick
  (params (ActionValue :type Boolean) (ElapsedSeconds :type Float%20%28double-precision%29) (TriggeredSeconds :type Float%20%28double-precision%29) (InputAction :type Input%20Action%20Object%20Reference :default "/Game/MyAssets/MainBP/Input/InputAction_RightClick.InputAction_RightClick"))
  ;[1 1 1] Right click
  (if (CallFunction|ActorinHand)
    (Default|CancelActualSpell (Variables|Default|GetAC_SystEco))
    (Variables|Default|SetPowerInHand 0)))

(event EventBeginPlay
  (bind _aspc_player (Utilities|Casting|CastToPC_Player (Pawn|GetController)))
  (bind _output_get (Variables|Default|SetPC_Player _aspc_player))
  (Pawn|Possess _output_get self)
  (Input|AddMappingContext (PlayerController|LocalPlayerSubsystems|GetEnhancedInputLocalPlayerSubsystem _output_get) "/Game/MyAssets/MainBP/Input/MC_BaseMovement.MC_BaseMovement" 0 "(bIgnoreAllPressedKeysUntilRelease=True,bForceImmediately=False,bNotifyUserSettings=False)")
  (Variables|/Script/Engine.PlayerController|SetbShowMouseCursor (Variables|Default|GetPC_Player) true)
  (bind _returnvalue (UserInterface|CreateWidget "/Game/MyAssets/MainBP/Widget/WB_HUD.WB_HUD_C"))
  (bind _output_get_2 (Variables|Default|SetWidgetHUD _returnvalue))
  (UserInterface|Viewport|AddtoViewport _output_get_2 0))

(event Input|KeyboardEvents|DebugKeyT
  (params (Key :type Key%20Structure :default "None") (ActionValue :type Input%20Action%20Value%20Structure))
  (:Pressed
    (Variables|/Game/MyAssets/MainBP/AC_SystEco.AC_SystEco_C|SetMoney (Variables|Default|GetAC_SystEco) 50)))

(event Input|MouseEvents|MouseWheelUp
  (params (Key :type Key%20Structure :default "None"))
  (bind _springarm (Variables|Default|GetSpringArm))
  ;[1 1 1] Zoom
  (:Pressed
    (Variables|/Script/Engine.SpringArmComponent|SetTargetArmLength _springarm (Math|Float|Clamp(Float) (- (Variables|/Script/Engine.SpringArmComponent|GetTargetArmLength _springarm) 4e+01) 1e+03 2e+03))))

(event Input|MouseEvents|MouseWheelDown
  (params (Key :type Key%20Structure :default "None"))
  (bind _springarm (Variables|Default|GetSpringArm))
  ;[1 1 1] Zoom
  (:Pressed
    (Variables|/Script/Engine.SpringArmComponent|SetTargetArmLength _springarm (Math|Float|Clamp(Float) (+ (Variables|/Script/Engine.SpringArmComponent|GetTargetArmLength _springarm) 4e+01) 1e+03 2e+03))))

(fn ConstructionScript)

(fn ActorinHand
  (return (Utilities|IsValid (Variables|Default|GetPowerInHand))))

(fn GetClickedActor
  (bind _pc_player (Variables|Default|GetPC_Player))
  (bind _hitresult (Game|Player|GetHitResultUnderCursorbyChannel _pc_player "TraceTypeQuery1" true))
  (bind (_bblockinghit _binitialoverlap _time _distance _location _impactpoint _normal _impactnormal _physmat _hitactor) (Collision|BreakHitResult _hitresult))
  (return _location _hitactor))